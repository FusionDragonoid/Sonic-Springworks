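; Playable Frenzy Wisp (PF) character that charges forward with random sideways lurches until its energy runs out, with a single launch jump until landing.
; An attached hit capsule deals damage, while overlapped objects receive an eat message and return values that fill an eat counter.
; Filling it raises the Frenzy level: a flickering grow pauses drain, enlarges body and hitbox, and changes walk speed.
; Springs and dash objects flag de-transform; balloons flag interaction.
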(event `self.OnLanded`
  (params (Hit :type "HitResult Structure (by ref)"))
  (set `self.CanJump?` true))

(event `InputAction|Jump` :paused true
  (params (Key :type "Key Structure"))
  (:`Pressed`
    (bind _w_pausescreen (`self.` (`self.PlayerControllerRef`))
      (:`false`
        (if (`self.CanJump?`)
          (`self.LaunchCharacter` (* (`self.GetActorUpVector`) (`self.FrenzyJumpPower`)) false true)
          (`GameplayStatics.PlaySound2D` "/Game/SonicSpringworks/Objects/Wisps/PF_Wisp/SFX/Phantom_Rodeo_Sjump.Phantom_Rodeo_Sjump" 1.0 1.0 0.0 null null)
          (set `self.CanJump?` false)))
      (:`true`
        (`self.Select_A` _w_pausescreen)))))

(event `self.ChildEnergy`
  (`GameplayStatics.PlaySound2D` "/Game/SonicSpringworks/Objects/Wisps/PF_Wisp/SFX/Phantom_Rodeo_Sjump.Phantom_Rodeo_Sjump" 1.0 1.0 0.0 null null)
  (`self.SpawnHitCapsule` (`self.Get Combat Actor`) (make `` "PF_Eat" 4 "None" (`KismetMathLibrary.MakeVector` (`SphereComponent.SphereRadius` (`self.EatRadius`)) (`CapsuleComponent.CapsuleHalfHeight` (`self.CapsuleComponent`))) (40.0 0.0 40.0) (struct :`Roll` 90.0) (1.0 1.0 1.0) 0.9 (1.0 0.0 0.0) 1200.0 0 0 0 1.0 0.4 0 5.0 0) 0 (`self.Mesh`) null null)
  (set `self.WEnergyDrain` (`self.PFEnergyDrain`))
  (set `self.WEnergyDrainMod` (`self.PFEnergyMod`))
  (bind _returnvalue (`KismetSystemLibrary.K2_SetTimerDelegate` (delegate `EnergyCheck`) 0.01 true))
  (set `self.EnergyTimer` _returnvalue)
  (bind _returnvalue_2 (`KismetSystemLibrary.K2_SetTimerDelegate` (delegate `RandomPull`) 0.1 true))
  (set `self.RandomTimer` _returnvalue_2))

(event `EnergyCheck`
  (if (<= (`self.WEnergyCurrent`) 0.0)
    (`KismetSystemLibrary.K2_ClearAndInvalidateTimerHandle` (`self.EnergyTimer`))
    (`KismetSystemLibrary.K2_ClearAndInvalidateTimerHandle` (`self.RandomTimer`))
    (`self.EnergyDrained`)
    (elif (<= (`self.CurrentSpeed`) 2000.0)
      (`self.AddMovementInput` (`self.GetActorForwardVector`)))))

(event `RandomPull`
  (`KismetSystemLibrary.Delay` (`KismetMathLibrary.RandomFloatInRange` 0.0 0.3))
  (`self.LaunchCharacter` (* (`self.GetActorRightVector`) (`KismetMathLibrary.FClamp` (* (`KismetMathLibrary.RandomFloatInRange` -0.6 0.6) (/ (`self.CurrentSpeed`) 1.3)) -2000.0 2000.0))))

(event `self.ReceiveBeginPlay`)

(event `self.EatRadius.OnComponentBeginOverlap`
  (params (OverlappedComponent :type "PrimitiveComponent Object Reference") (OtherActor :type "Actor Object Reference") (OtherComp :type "PrimitiveComponent Object Reference") (OtherBodyIndex :type Integer) (bFromSweep :type Boolean) (SweepResult :type "HitResult Structure (by ref)"))
  (if (`KismetSystemLibrary.DoesImplementInterface` OtherActor)
    (message `/Game/SonicSpringworks/Objects/Wisps/PF_Wisp/BP_PF_Wisp.WispEatObject` OtherActor self (`self.CurrentSize`) "Frenzy")))

(event `self.WispEatObjectInfo`
  (params (FrenzyEatValue :type "Float (double-precision)") (VoidEatValue :type "Float (double-precision)") (AsteroidEatValue :type "Float (double-precision)") (BombEatValue :type "Float (double-precision)"))
  (bind _ascombat_actor (`self.Get Combat Actor`))
  (bind _currentsize (`self.CurrentSize`))
  (bind _capsulecomponent (`self.CapsuleComponent`))
  (bind _growspeed (`self.GrowSpeed`))
  (bind _frenzylevel (`self.FrenzyLevel`))
  (bind _eatcount (`self.EatCount`))
  (bind _charactermovement (`self.CharacterMovement`))
  (bind _returnvalue (select `int` (`self.FrenzyLevel`) :`0` (1.0 1.0 1.0) :`1` (1.5 1.5 1.5) :`2` (2.0 2.0 2.0) :`3` (2.0 2.5 2.5) :!type "Vector Structure"))
  (set `self.EatCount` (+ FrenzyEatValue _eatcount))
  (`ActorComponent.Activate` (`self.Chomp`) true)
  (if (and (>= _eatcount (select `int` _frenzylevel :`0` 5.0 :`1` 7.0 :`2` 10.0)) (!= _frenzylevel 3))
    (set `self.EatCount` 0.0)
    (set `self.FrenzyLevel` (`KismetMathLibrary.Clamp` (+ (`self.FrenzyLevel`) 1) 0 3))
    (`MovementComponent.StopMovementImmediately` _charactermovement)
    (`GameplayStatics.PlaySound2D` "/Game/SonicSpringworks/Objects/Wisps/PF_Wisp/SFX/Phantom_Rodeo_Big.Phantom_Rodeo_Big" 1.0 1.0 0.0 null null)
    (set `self.WEnergyDrain` 0.0)
    (set `self.CanMoveX?` false)
    (set `self.CurrentSize` (`self.GetActorScale3D`))
    (`SceneComponent.SetWorldScale3D` _capsulecomponent _returnvalue)
    (`KismetSystemLibrary.Delay` _growspeed)
    (`SceneComponent.SetWorldScale3D` _capsulecomponent _currentsize)
    (`KismetSystemLibrary.Delay` _growspeed)
    (`SceneComponent.SetWorldScale3D` _capsulecomponent _returnvalue)
    (`KismetSystemLibrary.Delay` _growspeed)
    (`SceneComponent.SetWorldScale3D` _capsulecomponent _currentsize)
    (`KismetSystemLibrary.Delay` _growspeed)
    (`SceneComponent.SetWorldScale3D` _capsulecomponent _returnvalue)
    (set `self.CurrentSize` _returnvalue)
    (set `self.CanMoveX?` true)
    (set `self.WEnergyDrain` (`self.PFEnergyDrain`))
    (`self.ChangeHitbox_Size` _ascombat_actor (`KismetMathLibrary.MakeVector` (`SphereComponent.GetScaledSphereRadius` (`self.EatRadius`)) (`CapsuleComponent.GetScaledCapsuleHalfHeight` (`self.CapsuleComponent`))) "PF_Eat" 0)
    (`self.ChangeHitbox_Damage` _ascombat_actor (`KismetMathLibrary.FTrunc` (* (.x _returnvalue) 4.0)) "PF_Eat" 0)
    (set `CharacterMovementComponent.MaxWalkSpeed` (select `int` (`self.FrenzyLevel`) :`0` 5500.0 :`1` 4500.0 :`2` 3500.0 :`3` 2500.0) _charactermovement)))

(fn `CHILD ObjectInteract`
  (params (ObjectType :type Byte :default 0))
  (switch `|SwitchEnum` ObjectType
    (:`NewEnumerator0`
      (set `self.isObjectDeTransform?` true :!label _label)
      (set `self.isObjectInteract?` false)
      (set `self.isObjectRemove?` false))
    (:`NewEnumerator1`
      (goto _label))
    (:`NewEnumerator2`
      (goto _label))
    (:`NewEnumerator3`
      (goto _label))
    (:`NewEnumerator4`
      (set `self.isObjectDeTransform?` false)
      (set `self.isObjectInteract?` true)
      (set `self.isObjectRemove?` false))))

(fn `UserConstructionScript`)