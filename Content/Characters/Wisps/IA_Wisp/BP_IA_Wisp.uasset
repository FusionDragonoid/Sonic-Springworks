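; Asteroid Wisp character, a child wisp that eats objects via EatRadius overlaps to grow its radius and jump strength, with energy drain.
; Holding Jump charges while shrinking the radius; releasing launches it along its up vector and re-expands the radius.
; Holding Jump mid-air slows movement and falling by editing the physics volume's TerminalVelocity, which object interrupts restore.
; Timelines spin three asteroid rings, and Tick scales the main ring from EatRadius.
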(event `self.ReceiveBeginPlay`
  (`|ExecutionSequence`
    (:`then_0`
      (bind (_direction _time) (`Timeline|Timeline_0` :!via `PlayFromStart`)
        (:`Update`
          (`SceneComponent.K2_SetRelativeRotation` (`self.AsteroidRing`) (`KismetMathLibrary.MakeRotator` 0.0 (`KismetMathLibrary.SelectFloat` 90.0 0.0 (`self.Is2D?`)) _time) false false))))
    (:`then_1`
      (bind (_direction_2 _time_2) (`Timeline|Timeline_1` :!via `PlayFromStart`)
        (:`Update`
          (`SceneComponent.K2_SetRelativeRotation` (`self.AsteroidRing1`) (`KismetMathLibrary.MakeRotator` 0.0 0.0 _time_2) false false))))
    (:`then_2`
      (bind (_direction_3 _time_3) (`Timeline|Timeline_2` :!via `PlayFromStart`)
        (:`Update`
          (`SceneComponent.K2_SetRelativeRotation` (`self.AsteroidRing2`) (`KismetMathLibrary.MakeRotator` 0.0 0.0 _time_3) false false))))))

(event `self.ReceiveTick`
  (params (DeltaSeconds :type "Float (double-precision)"))
  (`SceneComponent.SetWorldScale3D` (`self.AsteroidRing`) (`KismetMathLibrary.VLerp` (1.5 1.5 1.5) (2.25 2.25 2.25) (/ (- (`SphereComponent.SphereRadius` (`self.EatRadius`)) 250.0) 250.0)))
  (if (`self.isObjectInterupt?`)
    (`/Engine/EditorBlueprintResources/StandardMacros.DoOnce` false :!label _label
      (:`Completed`
        (`KismetSystemLibrary.Delay` 1.0)
        (set `self.isObjectInterupt?` false)))
    (else
      (goto _label :!via `Reset`))))

(event `self.ChildEnergy`
  (set `self.WEnergyDrain` (`self.IAEnergyDrain`))
  (set `self.WEnergyDrainMod` (`self.IAEnergyMod`))
  (set `self.isCanJump?` true)
  (bind _returnvalue (`KismetSystemLibrary.K2_SetTimerDelegate` (delegate `EnergyCheck`) 0.01 true))
  (set `self.EnergyTimer` _returnvalue))

(event `EnergyCheck`
  (if (<= (`self.WEnergyCurrent`) 0.0)
    (`self.EnergyDrained`)
    (`KismetSystemLibrary.K2_ClearAndInvalidateTimerHandle` (`self.EnergyTimer`))))

(event `InputAction|Jump`
  (params (Key :type "Key Structure"))
  (bind _playercontrollerref (`self.PlayerControllerRef`))
  (bind _charactermovement (`self.CharacterMovement`))
  (bind _returnvalue (`MovementComponent.GetPhysicsVolume` _charactermovement))
  (:`Pressed`
    (bind _w_pausescreen (`self.` _playercontrollerref)
      (:`false`
        (if (`self.isObjectInterupt?`)
          _
          (elif (`self.isCanJump?`)
            (set `PhysicsVolume.TerminalVelocity` 300.0 _returnvalue)
            (bind _returnvalue_2 (`KismetSystemLibrary.K2_SetTimerDelegate` (delegate `ChargeJump`) 0.1 true))
            (set `self.IAJumpTimer` _returnvalue_2)
            (set `self.isCanJump?` false)
            (elif (`self.isJumpingIA`)
              (set `PhysicsVolume.TerminalVelocity` 300.0 _returnvalue)
              (set `CharacterMovementComponent.MaxWalkSpeed` 2500.0 _charactermovement)))))
      (:`true`
        (`self.Select_A` _w_pausescreen))))
  (:`Released`
    (`self.` _playercontrollerref
      (:`false`
        (set `PhysicsVolume.TerminalVelocity` 10000.0 _returnvalue)
        (set `CharacterMovementComponent.MaxWalkSpeed` 6000.0 _charactermovement)
        (if (not (`self.isJumpingIA`))
          (set `self.isJumpingIA` true)
          (`self.LaunchCharacter` (* (`self.GetActorUpVector`) (`self.IAJumpCharge`)) :!label _label_2)
          (set `self.IAJumpCharge` 0.0 :!label _label_3)
          (bind _returnvalue_3 (`KismetSystemLibrary.K2_SetTimerDelegate` (delegate `ExpandRadius`) 0.01 true))
          (set `self.ExpandRadiusTimer` _returnvalue_3))))))

(event `ChargeJump`
  (bind _returnvalue (`KismetMathLibrary.FClamp` (- (`self.IAJumpRadius`) (`self.RadiusShrinkRate`)) 250.0 3000.0))
  (if (`PlayerController.IsInputKeyDown` (`self.PlayerControllerRef`) (stale `InputAction|Jump` Key))
    (set `self.IAJumpCharge` (`KismetMathLibrary.FClamp` (+ (`self.IAJumpChargeRate`) (`self.IAJumpCharge`)) 300.0 (+ (`self.IAJumpChargeMax`) (* (`self.IAEatCurrent`) 0.2))))
    (set `self.isChargingJump` true)
    (`SphereComponent.SetSphereRadius` (`self.EatRadius`) _returnvalue true)
    (set `self.IAJumpRadius` _returnvalue)
    (if (`self.isObjectInterupt?`)
      (`KismetSystemLibrary.K2_ClearAndInvalidateTimerHandle` (`self.IAJumpTimer`))
      (goto _label_3))
    (else
      (`KismetSystemLibrary.K2_ClearAndInvalidateTimerHandle` (`self.IAJumpTimer`))
      (if (not (`self.isJumpingIA`))
        (set `self.isJumpingIA` true)
        (set `CharacterMovementComponent.MaxWalkSpeed` 6000.0 (`self.CharacterMovement`))
        (goto _label_2)))))

(event `ExpandRadius`
  (bind _returnvalue (`KismetMathLibrary.FClamp` (+ (`self.IAJumpRadius`) 5.0) 0.0 (`self.IAEatCurrent`)))
  (if (== (`self.IAJumpRadius`) (`self.IAEatCurrent`))
    (`KismetSystemLibrary.K2_ClearAndInvalidateTimerHandle` (`self.ExpandRadiusTimer`))
    (else
      (`SphereComponent.SetSphereRadius` (`self.EatRadius`) _returnvalue true)
      (set `self.IAJumpRadius` _returnvalue)
      (set `self.isChargingJump` false))))

(event `self.OnLanded`
  (params (Hit :type "HitResult Structure (by ref)"))
  (set `self.isCanJump?` true)
  (set `self.isJumpingIA` false))

(event `self.WispEatObjectInfo`
  (params (FrenzyEatValue :type "Float (double-precision)") (VoidEatValue :type "Float (double-precision)") (AsteroidEatValue :type "Float (double-precision)") (BombEatValue :type "Float (double-precision)"))
  (bind _output_get (set `self.IAEatCurrent` (`KismetMathLibrary.FClamp` (+ (* AsteroidEatValue 50.0) (`self.IAEatCurrent`)) 500.0 1300.0)))
  (set `self.CurrentSize` (`KismetMathLibrary.Conv_DoubleToVector` _output_get))
  (set `self.RadiusShrinkRate` (`KismetMathLibrary.FClamp` (+ (/ _output_get 180.0) (`self.RadiusShrinkRate`)) 15.0 150.0))
  (set `self.IAJumpChargeRate` (`KismetMathLibrary.FClamp` (+ (/ _output_get 200.0) (`self.IAJumpChargeRate`)) 100.0 300.0))
  (if (not (`self.isChargingJump`))
    (`SphereComponent.SetSphereRadius` (`self.EatRadius`) _output_get true)
    (set `self.IAJumpRadius` _output_get)))

(event `self.EatRadius.OnComponentBeginOverlap`
  (params (OverlappedComponent :type "PrimitiveComponent Object Reference") (OtherActor :type "Actor Object Reference") (OtherComp :type "PrimitiveComponent Object Reference") (OtherBodyIndex :type Integer) (bFromSweep :type Boolean) (SweepResult :type "HitResult Structure (by ref)"))
  (if (`KismetSystemLibrary.DoesImplementInterface` OtherActor)
    (message `/Game/Characters/Wisps/IA_Wisp/BP_IA_Wisp.WispEatObject` OtherActor self (`self.CurrentSize`) "Asteroid")))

(fn `CHILD ObjectInteract`
  (params (ObjectType :type Byte :default 0))
  (switch `|SwitchEnum` ObjectType
    (:`NewEnumerator0`
      _)
    (:`NewEnumerator1`
      _)
    (:`NewEnumerator2`
      _)
    (:`NewEnumerator3`
      _)
    (:`NewEnumerator4`
      _))
  (set `self.isObjectDeTransform?` false)
  (set `self.isObjectInteract?` true)
  (set `self.isObjectRemove?` false))

(fn `CHILD ObjectInterupt`
  (bind _charactermovement (`self.CharacterMovement`))
  (set `self.isObjectInterupt?` true)
  (set `self.isJumpingIA` false)
  (set `PhysicsVolume.TerminalVelocity` 10000.0 (`MovementComponent.GetPhysicsVolume` _charactermovement))
  (set `CharacterMovementComponent.MaxWalkSpeed` 6000.0 _charactermovement))

(fn `CHILD Spline Update`
  (params (`is2D?` :type Boolean))
  (if `is2D?`
    _))

(fn `CHILD_WarpRingRotation`
  (params (`isFlyingRing?` :type Boolean) (Rotation :type "Rotator Structure"))
  (if `isFlyingRing?`
    _))

(fn `UserConstructionScript`)